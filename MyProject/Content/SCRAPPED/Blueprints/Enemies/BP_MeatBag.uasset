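; BP_MeatBag is a scrapped enemy asset that acts as a damage readout, showing the damage it takes on a text render.
; Its damage handler calls HitTimer and adds each hit to DamageSum.
; HitTimer uses a short delay and the HasStartedHitTimer flag to batch hits, then displays and resets the total.
; BeginPlay also starts a looping timer at FireRateInSeconds, with no visible bound event.
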(event `self.ReceiveBeginPlay`
  (`KismetSystemLibrary.K2_SetTimerDelegate` :`Time` (`self.FireRateInSeconds`) :`bLooping` true)
  (add `Actor.OnTakeAnyDamage` (delegate `OnTakeAnyDamage_Event`)))

(event `OnTakeAnyDamage_Event`
  (params (DamagedActor :type "Actor Object Reference") (Damage :type "Float (single-precision)") (DamageType :type "DamageType Object Reference") (InstigatedBy :type "Controller Object Reference") (DamageCauser :type "Actor Object Reference"))
  (`self.HitTimer`)
  (set `self.DamageSum` (+ (`self.DamageSum`) Damage))
  (`self.HasStartedHitTimer?`
    (:`then`)
    (:`else`
      (set `self.HasStartedHitTimer?` true))))

(event `HitTimer`
  (`self.HasStartedHitTimer?`
    (:`then`)
    (:`else`
      (`KismetSystemLibrary.Delay` 0.1)
      (`TextRenderComponent.K2_SetText` (`self.TextRender`) (`KismetTextLibrary.Conv_DoubleToText` (`self.DamageSum`) "HalfToEven"))
      (set `self.DamageSum` 0.0)
      (set `self.HasStartedHitTimer?` false))))

(fn `UserConstructionScript`)