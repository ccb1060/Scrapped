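; BP_PickupItem is a pickup item actor, filed under SCRAPPED, that can be highlighted and report where it is.
; EnableHighlight and DisableHighlight set the IsHighlighted flag and toggle both custom depth rendering and the M_HighlightOverlay material on its static mesh.
; GetPickupLocation returns the actor's location, and all three functions print debug strings.
; It contains no pickup logic, and its event graph and construction scripts are empty.
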(fn `DisableHighlight`
  (set `self.bIsHighlighted` false)
  (`KismetSystemLibrary.PrintString` "Highlight: Disabled")
  (`PrimitiveComponent.SetRenderCustomDepth` (`self.StaticMesh`) false)
  (`MeshComponent.SetOverlayMaterial` (`self.StaticMesh`) null))

(fn `EnableHighlight`
  (set `self.bIsHighlighted` true)
  (`KismetSystemLibrary.PrintString` "Highlight: Enabled")
  (`PrimitiveComponent.SetRenderCustomDepth` (`self.StaticMesh`) true)
  (`MeshComponent.SetOverlayMaterial` (`self.StaticMesh`) "/Game/SCRAPPED/Materials/M_HighlightOverlay.M_HighlightOverlay"))

(fn `GetPickupLocation`
  (returns (ReturnValue :type "Vector Structure"))
  (`KismetSystemLibrary.PrintString` "GetPickupLocation called")
  (return (`self.K2_GetActorLocation`)))

(fn `UserConstructionScript`)

(fn `UserConstructionScript_0`)