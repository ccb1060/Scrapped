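; BP_MedKit is a health pickup that restores a fixed amount of health to the player on contact.
; When the first-person character overlaps its capsule, it adds to PlayerHealth, caps it at the maximum and plays a higher-pitched 2D sound.
; It then finds the WBP_Upgrades widget by class search to refresh its health display, and destroys itself.
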(event `self.Capsule.OnComponentBeginOverlap`
  (params (OverlappedComponent :type "PrimitiveComponent Object Reference") (OtherActor :type "Actor Object Reference") (OtherComp :type "PrimitiveComponent Object Reference") (OtherBodyIndex :type Integer) (bFromSweep :type Boolean) (SweepResult :type "HitResult Structure (by ref)"))
  (bind _asbp_first_person_character (cast `/Game/SCRAPPED/Blueprints/BP_FirstPersonCharacter` OtherActor))
  (bind _output_get (set `/Game/SCRAPPED/Blueprints/BP_FirstPersonCharacter.PlayerHealth` (+ (`/Game/SCRAPPED/Blueprints/BP_FirstPersonCharacter.PlayerHealth` _asbp_first_person_character) 15.0) _asbp_first_person_character))
  (if (> _output_get 100.0)
    (set `/Game/SCRAPPED/Blueprints/BP_FirstPersonCharacter.PlayerHealth` 100.0 _asbp_first_person_character))
  (`GameplayStatics.PlaySound2D` "/Game/SCRAPPED/Audio/SFX/Common.Common" 1.0 1.5 0.0 null null)
  (bind _foundwidgets (`WidgetBlueprintLibrary.GetAllWidgetsOfClass` "/Game/SCRAPPED/UI/WBP_Upgrades.WBP_Upgrades_C"))
  (`/Game/SCRAPPED/UI/WBP_Upgrades.UpdateHealth` (`|GetArrayItem` _foundwidgets))
  (`self.K2_DestroyActor`))

(fn `UserConstructionScript`)