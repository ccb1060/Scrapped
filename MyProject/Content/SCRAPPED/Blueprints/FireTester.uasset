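; FireTester is a scrapped test enemy that fires bullets and can drop an upgrade when damaged.
; A looping timer spawns EnemyBullet at FireShotSpot at the configured fire rate.
; Any damage triggers chained coin flips that spawn a spread-reduction, parry-window or speed upgrade at that spot, then destroy the actor.
; If all three flips fail, it drops nothing and stays alive.
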(event `self.ReceiveBeginPlay`
  (`KismetSystemLibrary.K2_SetTimerDelegate` (delegate `FireBullet`) (`self.FireRateInSeconds`) true)
  (add `self.OnTakeAnyDamage` (delegate `OnTakeAnyDamage_Event`)))

(event `OnTakeAnyDamage_Event` :!signature `self.OnTakeAnyDamage`
  (params (DamagedActor :type "Actor Object Reference") (Damage :type "Float (single-precision)") (DamageType :type "DamageType Object Reference") (InstigatedBy :type "Controller Object Reference") (DamageCauser :type "Actor Object Reference"))
  (if (`KismetMathLibrary.RandomBool`)
    (`|SpawnActorFromClass` "/Game/SCRAPPED/Blueprints/Upgrades/Common/BP_UpgradeReduceSpread.BP_UpgradeReduceSpread_C" (`SceneComponent.K2_GetComponentToWorld` (`self.FireShotSpot`)) "Undefined" "MultiplyWithRoot" null null)
    (`self.K2_DestroyActor` :!label _label)
    (elif (`KismetMathLibrary.RandomBool`)
      (`|SpawnActorFromClass` "/Game/SCRAPPED/Blueprints/Upgrades/Rare/BP_UpgradeParryWindow.BP_UpgradeParryWindow_C" (`SceneComponent.K2_GetComponentToWorld` (`self.FireShotSpot`)) "Undefined" "MultiplyWithRoot" null null)
      (goto _label)
      (elif (`KismetMathLibrary.RandomBool`)
        (`|SpawnActorFromClass` "/Game/SCRAPPED/Blueprints/Upgrades/Epic/BP_UpgradeIncreaseSpeed.BP_UpgradeIncreaseSpeed_C" (`SceneComponent.K2_GetComponentToWorld` (`self.FireShotSpot`)) "Undefined" "MultiplyWithRoot" null null)
        (goto _label)))))

(event `FireBullet`
  (`|SpawnActorFromClass` "/Game/SCRAPPED/Blueprints/EnemyBullet.EnemyBullet_C" (`SceneComponent.K2_GetComponentToWorld` (`self.FireShotSpot`)) "Undefined" "MultiplyWithRoot" null null))

(fn `UserConstructionScript`)