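; BP_LevelManager streams level instances in sequence as the player progresses, starting with the arena level at BeginPlay.
; Each registered transform spawns a BP_LevelLoader with a level ID that toggles between two values and binds its load-next-level event.
; That event unloads the active instance, loads the named level at the given location, and destroys the previous loader.
; A counter on the alternating ID tracks main level passes.
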(event `self.ReceiveBeginPlay`
  (bind (_boutsuccess _returnvalue) (`LevelStreamingDynamic.LoadLevelInstanceBySoftObjectPtr` "/Game/SCRAPPED/_Levels/ArenaLevel.ArenaLevel" (0.0 0.0 0.0) (struct) "" null))
  (set `self.ActiveLevel` _returnvalue))

(event `RegisterLevelLoaderPosition`
  (params (Transform :type "Transform Structure"))
  (bind _returnvalue (select `int` (`self.IDSwitcher`) :`0` 1 :`1` 0))
  (bind _activelevelloader (`self.ActiveLevelLoader`)
    (:`then`
      (set `self.PreviousLevelLoader` _activelevelloader))
    (:`else`
      _))
  (bind _output_get (set `self.IDSwitcher` _returnvalue))
  (bind _returnvalue_2 (`|SpawnActorFromClass` "/Game/SCRAPPED/Blueprints/BP_LevelLoader.BP_LevelLoader_C" Transform "Undefined" "MultiplyWithRoot" null _output_get null))
  (bind _output_get_2 (set `self.ActiveLevelLoader` _returnvalue_2))
  (add `/Game/SCRAPPED/Blueprints/BP_LevelLoader.LoadNextLevel` _output_get_2 (delegate `LoadNextArea`))
  ; Track how many times player goes thru main level
  (switch `int` _returnvalue
    (:`0`
      (`/Engine/EditorBlueprintResources/StandardMacros.IncrementInt` (`self.MainLevelCount`)))))

(event `LoadNextArea`
  (params (LevelName :type String) (SpawnLocation :type "Vector Structure"))
  (`LevelStreaming.SetIsRequestingUnloadAndRemoval` (`self.ActiveLevel`) true)
  (bind (_boutsuccess _returnvalue) (`LevelStreamingDynamic.LoadLevelInstance` LevelName SpawnLocation (struct) "" null))
  (set `self.ActiveLevel` _returnvalue)
  (bind _previouslevelloader (`self.PreviousLevelLoader`)
    (:`then`
      (`self.K2_DestroyActor` _previouslevelloader))
    (:`else`)))

(fn `UserConstructionScript`)