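; Player bullet projectile that damages what it hits, spawns a bullet-hole decal and destroys itself.
; Hits deal double damage when WasParried is true, and an optional hitmarker sound plays on Enemy-tagged actors.
; The construction script copies bounce and homing variables into ProjectileMovement and debug-prints them.
; SetParried only prints a one-time confirmation and does not set WasParried here.
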(event `SetParried`
  (`/Engine/EditorBlueprintResources/StandardMacros.DoOnce` false
    (:`Completed`
      (`KismetSystemLibrary.PrintString` "Player Bullet confirms Parry"))))

(event `self.ReceiveHit`
  (params (MyComp :type "PrimitiveComponent Object Reference") (Other :type "Actor Object Reference") (OtherComp :type "PrimitiveComponent Object Reference") (bSelfMoved :type Boolean) (HitLocation :type "Vector Structure") (HitNormal :type "Vector Structure") (NormalImpulse :type "Vector Structure") (Hit :type "HitResult Structure (by ref)"))
  (if (and (`self.hitMarker?`) (`self.ActorHasTag` Other "Enemy"))
    (`GameplayStatics.SpawnSound2D` "/Game/SCRAPPED/Audio/SFX/Hitmarker.Hitmarker" 0.2 1.0 0.0 null))
  (`GameplayStatics.ApplyDamage` Other (`KismetMathLibrary.SelectFloat` 2.0 1.0 (`self.wasParried?`)))
  (`|SpawnActorFromClass` "/Game/SCRAPPED/Decal/BP_BulletHoleDecal.BP_BulletHoleDecal_C" (`KismetMathLibrary.MakeTransform` HitLocation (`KismetMathLibrary.MakeRotFromX` HitNormal)) "Undefined" "MultiplyWithRoot" null null)
  (`self.K2_DestroyActor`))

(fn `UserConstructionScript`
  (bind _output_get (set `ProjectileMovementComponent.bShouldBounce` (`self.bouncingBullet?`) (`self.ProjectileMovement`)))
  (bind _output_get_2 (set `ProjectileMovementComponent.HomingTargetComponent` (`self.HomingTargetRef`) (`self.ProjectileMovement`)))
  (bind _output_get_3 (set `ProjectileMovementComponent.HomingAccelerationMagnitude` (`self.HomingStrength`) (`self.ProjectileMovement`)))
  (bind _output_get_4 (set `ProjectileMovementComponent.bIsHomingProjectile` (`self.homingBullet?`) (`self.ProjectileMovement`)))
  (`KismetSystemLibrary.PrintText` (`|FormatText` "Bounce? {B} \nHoming? {H} \nHTarget {T} \nHAM {HAM}" _output_get _output_get_4 _output_get_2 _output_get_3)))