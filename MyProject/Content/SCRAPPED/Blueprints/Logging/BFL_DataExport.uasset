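; Blueprint function library for data export, with one function that saves a debug message to a timestamped JSON file.
; ExportSimpleString packs the message and current time into an STDebugExport struct, converts it to a JSON string, then parses that into a JSON object.
; It writes the file to the project directory and returns success with the path, or failure with error text in FullPath.
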(fn `ExportSimpleString`
  (params (Message :type String) (BaseFilename :type String :default "OutputLog"))
  (returns (Success :type Boolean) (FullPath :type String))
  (locals (TimestampFormat :type Text :default "NSLOCTEXT(\"[EB7140981DA5F7790F96511D8D65F8B3]\", \"5BCF94FC4C793C35CB541BB6B5AE9FF8\", \"{0}_{1}_{2}_{3}_{4}_{5}\")") (JsonData :type "JsonObjectWrapper Structure"))
  (bind (_returnvalue_year _returnvalue_month _returnvalue_day _returnvalue_hour _returnvalue_minute _returnvalue_second) (`KismetMathLibrary.BreakDateTime` (`KismetMathLibrary.Now`)))
  (bind _returnvalue (`KismetTextLibrary.Conv_TextToString` (`|FormatText` (`local.TimestampFormat`) _returnvalue_year _returnvalue_month _returnvalue_day _returnvalue_hour _returnvalue_minute _returnvalue_second)))
  (bind _returnvalue_2 (`KismetStringLibrary.Concat_StrStr` (`KismetSystemLibrary.GetProjectDirectory`) BaseFilename "_" _returnvalue ".json"))
  (bind (_outjsonstring _returnvalue_3) (`|StructToJsonString` (make `/Game/SCRAPPED/Blueprints/Logging/ST_DebugExport` Message _returnvalue)))
  (if _returnvalue_3
    (bind (_outjsonobject _returnvalue_4) (`JsonBlueprintFunctionLibrary.FromString` _outjsonstring))
    (if _returnvalue_4
      (bind _returnvalue_5 (`JsonBlueprintFunctionLibrary.ToFile` _outjsonobject (make `FilePath` _returnvalue_2)))
      (if _returnvalue_5
        (return true _returnvalue_2)
        (else
          (return false "Unable to convert JSON String to JSON Object")))
      (else
        (return false "Unable to convert JSON String to JSON Object")))
    (else
      (return false "Unable to convert data object to JSON String"))))