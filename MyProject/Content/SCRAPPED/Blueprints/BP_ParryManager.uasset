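; BP_ParryManager is a scrapped manager that plays a parry effect through post-process settings and then unpauses the game.
; On BeginPlay it finds a PostProcessVolume and caches its default settings.
; Tick watches ReadytoUnpause, clears it and calls StartParry.
; StartParry applies the parry settings, waits through a short Delay, then unpauses and restores the default look.
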(event `self.ReceiveBeginPlay`
  (bind _returnvalue (`GameplayStatics.GetActorOfClass` "/Script/Engine.PostProcessVolume"))
  (bind _output_get (set `self.PPRef` _returnvalue))
  (set `self.PPDefaultSettings` (`PostProcessVolume.Settings` _output_get)))

(event `self.ReceiveTick`
  (params (DeltaSeconds :type "Float (single-precision)"))
  (`self.readytoUnpause`
    (:`then`
      (set `self.readytoUnpause` false)
      (`self.StartParry`)
      (`KismetSystemLibrary.PrintString` "Unpausing" true true (struct :`R` 0.000525 :`G` 1.0 :`B` 0.151359 :`A` 1.0)))
    (:`else`)))

(event `StartParry`
  (set `PostProcessVolume.Settings` (`self.PPParrySettings`) (`self.PPRef`))
  (`KismetSystemLibrary.Delay` 0.5)
  (`GameplayStatics.SetGamePaused` false)
  (set `PostProcessVolume.Settings` (`self.PPDefaultSettings`) (`self.PPRef`)))

(fn `UserConstructionScript`)