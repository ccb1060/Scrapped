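; BP_LevelLoader is a two-door transition actor that seals the first-person player in while the next level loads.
; The previous door starts hidden; entering HitBox closes it and calls LoadNextLevel with a level name and X/Y spawn point from OffsetArray at LevelID, relative to the actor.
; After a short fixed delay, without checking load completion, the next door opens.
; Overlapping LeftLoaderBox closes that door behind the player.
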(event `self.ReceiveBeginPlay`
  (bind _doorprevious (`self.DoorPrevious`))
  (`SceneComponent.SetHiddenInGame` _doorprevious true false)
  (`PrimitiveComponent.SetCollisionEnabled` _doorprevious "NoCollision"))

(event `self.HitBox.OnComponentBeginOverlap`
  (params (OverlappedComponent :type "PrimitiveComponent Object Reference") (OtherActor :type "Actor Object Reference") (OtherComp :type "PrimitiveComponent Object Reference") (OtherBodyIndex :type Integer) (bFromSweep :type Boolean) (SweepResult :type "HitResult Structure (by ref)"))
  (bind _doorprevious (`self.DoorPrevious`))
  (bind _doornext (`self.DoorNext`))
  (bind (_output_levelname _output_locationvector) (break `/Game/SCRAPPED/Data/LevelandOffset` (`|GetArrayItem` (`self.OffsetArray`) (`self.LevelID`))))
  (bind (_returnvalue_x _returnvalue_y) (`KismetMathLibrary.BreakVector` (+ _output_locationvector (`self.K2_GetActorLocation`))))
  (cast `/Game/SCRAPPED/Blueprints/BP_FirstPersonCharacter` OtherActor)
  (`SceneComponent.SetHiddenInGame` _doorprevious false false)
  (`PrimitiveComponent.SetCollisionEnabled` _doorprevious "QueryAndPhysics")
  (`self.LoadNextLevel` _output_levelname (`KismetMathLibrary.MakeVector` _returnvalue_x _returnvalue_y))
  (`KismetSystemLibrary.Delay` 0.5)
  (`SceneComponent.SetHiddenInGame` _doornext true false)
  (`PrimitiveComponent.SetCollisionEnabled` _doornext "NoCollision"))

(event `self.LeftLoaderBox.OnComponentBeginOverlap`
  (params (OverlappedComponent :type "PrimitiveComponent Object Reference") (OtherActor :type "Actor Object Reference") (OtherComp :type "PrimitiveComponent Object Reference") (OtherBodyIndex :type Integer) (bFromSweep :type Boolean) (SweepResult :type "HitResult Structure (by ref)"))
  (bind _doornext (`self.DoorNext`))
  (cast `/Game/SCRAPPED/Blueprints/BP_FirstPersonCharacter` OtherActor)
  (`SceneComponent.SetHiddenInGame` _doornext false false)
  (`PrimitiveComponent.SetCollisionEnabled` _doornext "QueryAndPhysics"))

(fn `UserConstructionScript`)