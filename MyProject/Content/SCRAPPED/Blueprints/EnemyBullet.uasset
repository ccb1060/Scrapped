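; Enemy projectile that damages whatever it hits and can be parried toward a new aim point.
; On hit it applies a small fixed damage, spawns a bullet hole decal aligned to the surface normal and destroys itself.
; SetParrried redirects the ProjectileMovement velocity toward the supplied point at the supplied speed, gated by DoOnce.
; The deprecated SetParriedOLD instead rotates the sphere and reverses the velocity.
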(event `self.ReceiveHit`
  (params (MyComp :type "PrimitiveComponent Object Reference") (Other :type "Actor Object Reference") (OtherComp :type "PrimitiveComponent Object Reference") (bSelfMoved :type Boolean) (HitLocation :type "Vector Structure") (HitNormal :type "Vector Structure") (NormalImpulse :type "Vector Structure") (Hit :type "HitResult Structure (by ref)"))
  ; Event Hit
  (`GameplayStatics.ApplyDamage` Other 5.0)
  (`|SpawnActorFromClass` "/Game/SCRAPPED/Decal/BP_BulletHoleDecal.BP_BulletHoleDecal_C" (`KismetMathLibrary.MakeTransform` HitLocation (`KismetMathLibrary.MakeRotFromX` HitNormal)) "Undefined" "MultiplyWithRoot" null null)
  (`self.K2_DestroyActor`))

(event `SetParriedOLD`
  (params (ParryAim :type "Rotator Structure"))
  (bind _projectilemovement (`self.ProjectileMovement`))
  ; Depricated
  (`/Engine/EditorBlueprintResources/StandardMacros.DoOnce` false
    (:`Completed`
      (`KismetSystemLibrary.PrintString` "Enemy Bullet confirms Parry")
      (`SceneComponent.K2_SetWorldRotation` (`self.Sphere`) ParryAim false false)
      (set `MovementComponent.Velocity` (* (`MovementComponent.Velocity` _projectilemovement) -1.0) _projectilemovement))))

(event `SetParrried`
  (params (ParryAimPoint :type "Vector Structure") (ParriedBulletSpeed :type "Float (double-precision)"))
  ; Parried
  (`/Engine/EditorBlueprintResources/StandardMacros.DoOnce` false
    (:`Completed`
      (`KismetSystemLibrary.PrintString` "Enemy Bullet confirms Parry")
      (set `MovementComponent.Velocity` (* (`KismetMathLibrary.Normal` (- ParryAimPoint (`self.K2_GetActorLocation`))) ParriedBulletSpeed) (`self.ProjectileMovement`)))))

(fn `UserConstructionScript`)