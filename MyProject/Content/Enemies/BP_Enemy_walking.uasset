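; Walking enemy that takes damage, printing its remaining HP, and spawns a Niagara effect before destroying itself when health runs out.
; A looping timer started on BeginPlay regularly runs a player distance check and writes InAttackRange to the AI controller's Blackboard.
; The logic that would set the player as the Blackboard's TargetActor is disconnected and never runs.
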(event `self.ReceiveAnyDamage`
  (params (Damage :type "Float (single-precision)") (DamageType :type "DamageType Object Reference") (InstigatedBy :type "Controller Object Reference") (DamageCauser :type "Actor Object Reference"))
  (set `self.Health` (- (`self.Health`) Damage))
  (if (<= (`self.Health`) 0.0)
    (`NiagaraFunctionLibrary.SpawnSystemAtLocation` null (`self.K2_GetActorLocation`))
    (`self.K2_DestroyActor`)
    (else
      (`KismetSystemLibrary.PrintString` (`KismetStringLibrary.Concat_StrStr` "HP:" (`KismetStringLibrary.Conv_DoubleToString` (`self.Health`)))))))

(event `CheckDistance`
  (bind _returnvalue (`AIBlueprintHelperLibrary.GetBlackboard` (`AIBlueprintHelperLibrary.GetAIController` null)))
  (`/Engine/EditorBlueprintResources/StandardMacros.IsValid` _returnvalue
    (:`Is Valid`
      (`BlackboardComponent.SetValueAsBool` _returnvalue "InAttackRange" (< (`self.GetDistanceTo` (`GameplayStatics.GetPlayerCharacter` 0) null) 150.0)))))

(event `self.ReceiveBeginPlay`
  (`KismetSystemLibrary.K2_SetTimerDelegate` (delegate `CheckDistance`) 0.2 true))

(fn `UserConstructionScript`)