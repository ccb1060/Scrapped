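; Melee enemy Blueprint that plays an attack montage and deals damage to a pawn in front of it.
; TriggerMeleeAttack only starts the montage, while ExecuteAttack separately performs the hit check; neither event's caller is in this graph.
; ExecuteAttack prints a debug string, sphere-traces forward from slightly above the actor's origin for Pawn objects, and applies fixed damage to the first hit.
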(event `self.ExecuteAttack`
  (bind _returnvalue (+ (`self.K2_GetActorLocation` self) (0.0 0.0 50.0)))
  (`KismetSystemLibrary.PrintString` "Hello")
  (bind (_outhit _returnvalue_2) (`KismetSystemLibrary.SphereTraceSingleForObjects` _returnvalue (+ (* (`self.GetActorForwardVector` self) (150.0 150.0 150.0)) _returnvalue) 0.0 (`|MakeArray` "ObjectTypeQuery3" :!type "EObjectTypeQuery Enum")))
  (if _returnvalue_2
    (`GameplayStatics.ApplyDamage` (`.HitActor` (`GameplayStatics.BreakHitResult` _outhit)) 5.0 null self)))

(event `TriggerMeleeAttack`
  (`self.PlayAnimMontage` "/Game/Enemies/Sword_enemy/AM_MeleeAttack.AM_MeleeAttack"))

(fn `UserConstructionScript`
  (`parent.UserConstructionScript`))