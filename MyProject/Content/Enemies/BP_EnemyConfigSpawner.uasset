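; An enemy wave spawner actor that spawns configured enemy classes around itself on a repeating timer.
; One second after BeginPlay it spawns the first wave and starts a looping timer at the wave interval.
; Each wave spawns every class in the config map by its count scaled by difficulty and wave number, truncated to an integer.
; Spawns land at random reachable navmesh points within the spawn radius.
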(event `self.ReceiveBeginPlay`
  (`KismetSystemLibrary.Delay` 1.0)
  (`KismetSystemLibrary.K2_SetTimerDelegate` (delegate `SpawnNextWave`) (`self.WaveInterval`) true)
  (`self.SpawnNextWave`))

(event `SpawnNextWave`
  (bind _keys (`BlueprintMapLibrary.Map_Keys` (`self.EnemySpawnConfig`)))
  (for _array_element _keys
    (for _ (range 1 (+ (`KismetMathLibrary.FTrunc` (* (`BlueprintMapLibrary.Map_Find` (`self.EnemySpawnConfig`) _array_element) (`self.DifficultyMutiplier`) (`self.CurrentWave`))) 1))
      (`|SpawnActorFromClass` _array_element (`KismetMathLibrary.Conv_VectorToTransform` (`NavigationSystemV1.K2_GetRandomReachablePointInRadius` (`self.K2_GetActorLocation`) (`self.SpawnRadius`) null null)) "AdjustIfPossibleButAlwaysSpawn" "MultiplyWithRoot" null null)))
  (set `self.CurrentWave` (+ (`self.CurrentWave`) 1)))

(fn `UserConstructionScript`)