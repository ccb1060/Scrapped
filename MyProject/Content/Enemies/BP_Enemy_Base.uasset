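; Base enemy Blueprint with health, death and an attack-range check for AI.
; Any damage reduces Health, and at zero it spawns a particle or effect system at its location and destroys itself.
; After possession, a looping timer writes whether the player is within AttackRange to the InAttackRange Blackboard key.
; ExecuteAttack is an empty event.
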(event `self.ReceiveAnyDamage`
  (params (Damage :type "Float (single-precision)") (DamageType :type "DamageType Object Reference") (InstigatedBy :type "Controller Object Reference") (DamageCauser :type "Actor Object Reference"))
  (set `self.Health` (- (`self.Health`) Damage))
  (if (<= (`self.Health`) 0.0)
    (`NiagaraFunctionLibrary.SpawnSystemAtLocation` null (`self.K2_GetActorLocation`))
    (`self.K2_DestroyActor`)))

(event `CheckDistance`
  (bind _returnvalue (`AIBlueprintHelperLibrary.GetBlackboard` (`AIBlueprintHelperLibrary.GetAIController` self)))
  (`/Engine/EditorBlueprintResources/StandardMacros.IsValid` _returnvalue
    (:`Is Valid`
      (`BlackboardComponent.SetValueAsBool` _returnvalue "InAttackRange" (< (`self.GetDistanceTo` (`GameplayStatics.GetPlayerCharacter` 0) self) (`self.AttackRange`))))))

(event `self.ReceivePossessed`
  (params (NewController :type "Controller Object Reference"))
  (`KismetSystemLibrary.Delay` 0.1)
  (`KismetSystemLibrary.K2_SetTimerDelegate` (delegate `CheckDistance`) 0.2 true))

(event `self.ReceiveBeginPlay`)

(event `ExecuteAttack`)

(fn `UserConstructionScript`)