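; BP_ArenaTrigger is a box trigger that switches arena spawners on and off as the first-person player character enters and leaves it.
; Begin overlap calls ActivateArena for valid entries in TargetSpawner, and end overlap calls DeactivateArena, each printing a debug string.
; A DoOnce guards activation but resets inside the same loop, so it re-arms immediately whenever a valid spawner is found.
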(event `self.Box.OnComponentBeginOverlap`
  (params (OverlappedComponent :type "PrimitiveComponent Object Reference") (OtherActor :type "Actor Object Reference") (OtherComp :type "PrimitiveComponent Object Reference") (OtherBodyIndex :type Integer) (bFromSweep :type Boolean) (SweepResult :type "HitResult Structure (by ref)"))
  (bind _targetspawner (`self.TargetSpawner`))
  (cast `/Game/SCRAPPED/Blueprints/BP_FirstPersonCharacter` OtherActor)
  (`/Engine/EditorBlueprintResources/StandardMacros.DoOnce` false :!label _label
    (:`Completed`
      (for _array_element _targetspawner
        (`/Engine/EditorBlueprintResources/StandardMacros.IsValid` _array_element
          (:`Is Valid`
            (`/Game/Enemies/BP_EnemyConfigSpawner.ActivateArena` _targetspawner)
            (`KismetSystemLibrary.PrintString` "active")
            (goto _label :!via `Reset`)))))))

(event `self.Box.OnComponentEndOverlap`
  (params (OverlappedComponent :type "PrimitiveComponent Object Reference") (OtherActor :type "Actor Object Reference") (OtherComp :type "PrimitiveComponent Object Reference") (OtherBodyIndex :type Integer))
  (bind _targetspawner (`self.TargetSpawner`))
  (cast `/Game/SCRAPPED/Blueprints/BP_FirstPersonCharacter` OtherActor)
  (for _array_element _targetspawner
    (`/Engine/EditorBlueprintResources/StandardMacros.IsValid` _array_element
      (:`Is Valid`
        (`/Game/Enemies/BP_EnemyConfigSpawner.DeactivateArena` _targetspawner)
        (`KismetSystemLibrary.PrintString` "deactive")))))

(fn `UserConstructionScript`)